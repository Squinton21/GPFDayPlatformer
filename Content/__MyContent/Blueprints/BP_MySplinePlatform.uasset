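; Platform actor that travels along a spline once a ThirdPersonCharacter overlaps its trigger box.
; The overlap plays a timeline whose SplineDistance value, scaled by spline length, sets the platform mesh's world location without sweeping.
; The same distance drives the mesh's relative rotation from the spline, using only roll and yaw.
; The construction script applies the configurable static mesh and material to the platform.
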(event OnComponentBeginOverlap(Box)
  (params (OverlappedComponent :type Primitive%20Component%20Object%20Reference) (OtherActor :type Actor%20Object%20Reference) (OtherComp :type Primitive%20Component%20Object%20Reference) (OtherBodyIndex :type Integer) (bFromSweep :type Boolean) (SweepResult :type Hit%20Result%20Structure%20%28by%20ref%29))
  (bind _spline (Variables|Default|GetSpline))
  (bind _platform_mesh (Variables|Default|GetPlatform%20Mesh))
  (Utilities|Casting|CastToThirdPersonCharacter OtherActor)
  (bind _spline_distance (Timeline|Motion%20Timeline Play)
    (:Update
      (Transformation|SetWorldLocation _platform_mesh (Spline|GetLocationatDistanceAlongSpline _spline (* _spline_distance (Spline|GetSplineLength _spline)) "World") false false)
      (Transformation|SetRelativeRotation _platform_mesh (Math|Rotator|MakeRotator (.roll (Spline|GetRotationatDistanceAlongSpline _spline (* _spline_distance (Spline|GetSplineLength _spline)) "Local")) 0.0 (.yaw (Spline|GetRotationatDistanceAlongSpline _spline (* _spline_distance (Spline|GetSplineLength _spline)) "Local"))) false false))))

(fn ConstructionScript
  (bind _platform_mesh (Variables|Default|GetPlatform%20Mesh))
  (Components|StaticMesh|SetStaticMesh _platform_mesh (Variables|Default|GetStatic%20Mesh))
  (Rendering|Material|SetMaterial _platform_mesh 0 (Variables|Default|GetMaterial)))